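; Destructible ice floor grid whose tiles take damage from hammer hits and player melt events, stepping through cube states to melted.
; MapData stores each tile's state and damage; exceeding MaximumDamage advances the state.
; Each drawn state gets an instanced mesh bucket holding every tile, so state changes just shift instance Z between zero and RemovalHeight, keeping indices stable.
; The construction script's preview grid is cleared at BeginPlay.
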(event `self.ReceiveBeginPlay`
  (`InstancedStaticMeshComponent.ClearInstances` (`self.MapSize`))
  (`self.GenerateTestMap`)
  (`self.BucketGeneration`)
  (`self.GenerateInitalMesh`)
  (add `self.HammerTime` (delegate `HammerTime_Event`))
  (add `self.PlayerMelt` (delegate `PlayerMelt_Event`)))

(event `HammerTime_Event`
  (params (HammerHitLoc :type "Vector Structure"))
  (bind _tile_index (`self.GetTileIndexFromLocation` HammerHitLoc))
  (`self.DamageTile` _tile_index (`self.HammerDamage`)))

(event `PlayerMelt_Event`
  (params (PlayerLoc :type "Vector Structure"))
  (bind _tile_index (`self.GetTileIndexFromLocation` PlayerLoc))
  (`self.DamageTile` _tile_index (`self.StandDamage`)))

(fn `AddInstance`
  (params (Bucket :type "/Game/Blueprints/BPS_TileBucket Structure") (`Tile Loc` :type "IntPoint Structure"))
  (bind ((`InstancedMeshComponent_9_15013CAC4C513ECB4D65FB8969B052F8` _instancedmeshcomponent)) (break `/Game/Blueprints/BPS_TileBucket` Bucket))
  (bind _index (`self.CalculateIndex` `Tile Loc`))
  (`/Engine/EditorBlueprintResources/StandardMacros.IsValid` _instancedmeshcomponent
    (:`Is Valid`
      (`InstancedStaticMeshComponent.UpdateInstanceTransform` _instancedmeshcomponent _index (`KismetMathLibrary.MakeTransform` (`KismetMathLibrary.MakeVector` (.x (.location (`InstancedStaticMeshComponent.GetInstanceTransform` _instancedmeshcomponent _index false))) (.y (.location (`InstancedStaticMeshComponent.GetInstanceTransform` _instancedmeshcomponent _index false)))) (.rotation (`InstancedStaticMeshComponent.GetInstanceTransform` _instancedmeshcomponent _index false)) (.scale (`InstancedStaticMeshComponent.GetInstanceTransform` _instancedmeshcomponent _index false))) false true true))))

(fn `BucketGeneration`
  (bind _enumvalue (foreach `/Game/Blueprints/BPE_IceState`)
    (:`LoopBody`
      (bind ((`State_20_C6E0F3984BD6CDFB172EC696CBA47F35` _state) (`StateMesh_2_BD42902149124139DA4A8DA67872F008` _statemesh) (`StateMaterial_6_464E49D349390572013184AB0101E15B` _statematerial) (`IsDrawn_17_F765C21744ACDBDEC1F79C925591F274` _isdrawn)) (break `/Game/Blueprints/BPS_TileBucket` (`|GetArrayItem` (`self.TileBuckets`) (`KismetMathLibrary.Conv_ByteToInt` _enumvalue))))
      (if _isdrawn
        (bind _returnvalue (`AddComponent|NODE_AddInstancedStaticMeshComponent-0`))
        (`StaticMeshComponent.SetStaticMesh` _returnvalue _statemesh)
        (`PrimitiveComponent.SetMaterial` _returnvalue 0 _statematerial)
        (`SceneComponent.K2_AttachToComponent` _returnvalue (`self.IceSegments`) "None" "SnapToTarget" "SnapToTarget" "SnapToTarget" true)
        (`KismetArrayLibrary.Array_Set` (`self.TileBuckets`) (`KismetMathLibrary.Conv_ByteToInt` _state) (make `/Game/Blueprints/BPS_TileBucket` _state _statemesh _statematerial _returnvalue))))))

(fn `CalculateIndex`
  (params (`Tile Pos` :type "IntPoint Structure"))
  (returns (Index :type Integer))
  (bind (_x _y) (break `IntPoint` `Tile Pos`))
  (return (+ _x (* _y (`.X` (break `IntPoint` (`self.Ice Map Size`)))))))

(fn `CalculateTileLocation`
  (params (TileLoc :type "IntPoint Structure"))
  (returns (TileTransform :type "Transform Structure"))
  (bind (_x _y) (break `IntPoint` TileLoc))
  (bind (_x_2 _y_2) (break `IntPoint` (`self.Ice Map Size`)))
  (bind _x_3 (.x (`self.Ice Cube Mesh Dimention`)))
  (bind _y_3 (.y (`self.Ice Cube Mesh Dimention`)))
  (return (`KismetMathLibrary.Conv_VectorToTransform` (`KismetMathLibrary.MakeVector` (+ (- (* _x _x_3) (/ (* _x_2 _x_3) 2.0)) (/ _x_3 2.0)) (+ (- (* _y _y_3) (/ (* _y_2 _y_3) 2.0)) (/ _y_3 2.0))))))

(fn `DamageTile`
  (params (TilePosition :type "IntPoint Structure") (Damage :type "Float (double-precision)"))
  (bind (_x _y) (break `IntPoint` TilePosition))
  (bind (_valid _tiledata) (`self.GetTileData` TilePosition))
  (if _valid
    (bind (_state _position _totaldamage) (break `/Game/Blueprints/BPS_IceTile` _tiledata))
    (bind _returnvalue (+ Damage _totaldamage))
    (if (> _returnvalue (`self.MaximumDamage`))
      (bind (_newicestate _newbucket _oldbucket) (`self.GetNextIceState` _state))
      (`self.AddInstance` _newbucket _position)
      (`self.RemoveInstance` _oldbucket _position)
      (`self.SetTileData` _position (make `/Game/Blueprints/BPS_IceTile` _newicestate _position))
      (else
        (`self.SetTileData` _position (make `/Game/Blueprints/BPS_IceTile` _state _position _returnvalue))))
    (else
      (`KismetSystemLibrary.PrintString` (`KismetStringLibrary.Concat_StrStr` "TileDamage: Invalid Tile (" (`KismetStringLibrary.Conv_IntToString` _x) " : " (`KismetStringLibrary.Conv_IntToString` _y) ")")))))

(fn `GenerateInitalMesh`
  (bind _mapdata (`self.MapData`))
  (bind (_x _y) (break `IntPoint` (`self.Ice Map Size`)))
  (`|ExecutionSequence`
    (:`then_0`
      ;[1 1 1] Distribute Into Buckets
      (for (_array_element _array_index) _mapdata
        (bind (_state _position) (break `/Game/Blueprints/BPS_IceTile` _array_element))
        (if (`.IsDrawn_17_F765C21744ACDBDEC1F79C925591F274` (break `/Game/Blueprints/BPS_TileBucket` (`|GetArrayItem` (`self.TileBuckets`) (`KismetMathLibrary.Conv_ByteToInt` _state))))
          (`KismetArrayLibrary.Array_Set` _mapdata _array_index (make `/Game/Blueprints/BPS_IceTile` _state _position) true))))
    (:`then_1`
      ;[1 1 1] Generate Tile Instances
      (bind _enumvalue (foreach `/Game/Blueprints/BPE_IceState`)
        (:`LoopBody`
          (bind ((`InstancedMeshComponent_9_15013CAC4C513ECB4D65FB8969B052F8` _instancedmeshcomponent) (`IsDrawn_17_F765C21744ACDBDEC1F79C925591F274` _isdrawn)) (break `/Game/Blueprints/BPS_TileBucket` (`|GetArrayItem` (`self.TileBuckets`) (`KismetMathLibrary.Conv_ByteToInt` _enumvalue))))
          (if _isdrawn
            (for _index (range _y)
              (for _index_2 (range _x)
                (bind _intpoint (make `IntPoint` _index_2 _index))
                (bind _index_3 (`self.CalculateIndex` _intpoint))
                (bind _tiletransform (`self.CalculateTileLocation` _intpoint))
                (`InstancedStaticMeshComponent.AddInstance` _instancedmeshcomponent (`KismetMathLibrary.MakeTransform` (`KismetMathLibrary.MakeVector` (.x (.location _tiletransform)) (.y (.location _tiletransform)) (select `bool` (`|EnumEquality` (`.State_7_25813F964726E9687C2E05B5FFACDAAC` (break `/Game/Blueprints/BPS_IceTile` (`|GetArrayItem` (`self.MapData`) _index_3))) _enumvalue) :`false` (`self.RemovalHeight`))) (.rotation _tiletransform) (.scale _tiletransform)))))))))))

(fn `GenerateTestMap`
  (locals (NextState :type "/Game/Blueprints/BPE_IceState Enum"))
  (bind (_x _y) (break `IntPoint` (`self.Ice Map Size`)))
  (for _index (range _y)
    (for _index_2 (range _x)
      (bind _intpoint (make `IntPoint` _index_2 _index))
      (`self.SetTileData` _intpoint (make `/Game/Blueprints/BPS_IceTile` (`local.NextState`) _intpoint)))))

(fn `GetNextIceState`
  (params (OldIceState :type "/Game/Blueprints/BPE_IceState Enum" :default "NewEnumerator0"))
  (returns (NewIceState :type "/Game/Blueprints/BPE_IceState Enum") (NewBucket :type "/Game/Blueprints/BPS_TileBucket Structure") (OldBucket :type "/Game/Blueprints/BPS_TileBucket Structure"))
  (bind _tilebuckets (`self.TileBuckets`))
  (bind _output (`|GetArrayItem` _tilebuckets 3))
  (bind _output_2 (`|GetArrayItem` _tilebuckets 4))
  (bind _output_3 (`|GetArrayItem` _tilebuckets 5))
  (bind _output_4 (`|GetArrayItem` _tilebuckets 6))
  (bind _output_5 (`|GetArrayItem` _tilebuckets 2))
  (bind _output_6 (`|GetArrayItem` _tilebuckets 1))
  (return (select `/Game/Blueprints/BPE_IceState` OldIceState :`NewEnumerator0` "NewEnumerator1" :`NewEnumerator1` "NewEnumerator2" :`NewEnumerator2` "NewEnumerator3" :`NewEnumerator3` "NewEnumerator4" :`NewEnumerator4` "NewEnumerator5" :`NewEnumerator5` "NewEnumerator6" :`NewEnumerator6` "NewEnumerator6" :!type "/Game/Blueprints/BPE_IceState Enum") (select `/Game/Blueprints/BPE_IceState` OldIceState :`NewEnumerator0` _output_6 :`NewEnumerator1` _output_5 :`NewEnumerator2` _output :`NewEnumerator3` _output_2 :`NewEnumerator4` _output_3 :`NewEnumerator5` _output_4 :`NewEnumerator6` _output_4) (select `/Game/Blueprints/BPE_IceState` OldIceState :`NewEnumerator0` (`|GetArrayItem` _tilebuckets) :`NewEnumerator1` _output_6 :`NewEnumerator2` _output_5 :`NewEnumerator3` _output :`NewEnumerator4` _output_2 :`NewEnumerator5` _output_3 :`NewEnumerator6` _output_4)))

(fn `GetTileData`
  (params (TilePosition :type "IntPoint Structure"))
  (returns (Valid :type Boolean) (TileData :type "/Game/Blueprints/BPS_IceTile Structure") (Index :type Integer))
  (bind _mapdata (`self.MapData`))
  (bind _index (`self.CalculateIndex` TilePosition))
  (if (`KismetArrayLibrary.Array_IsValidIndex` _mapdata _index)
    (return true (`|GetArrayItem` _mapdata _index) _index)
    (else
      (return false (struct) _index))))

(fn `GetTileIndexFromLocation`
  (params (`Tile Loc` :type "Vector Structure"))
  (returns (`Tile Index` :type "IntPoint Structure"))
  (bind (_x _y) (break `IntPoint` (`self.Ice Map Size`)))
  (return (make `IntPoint` (`KismetMathLibrary.FFloor` (+ (/ (.x `Tile Loc`) (.x (`self.Ice Cube Mesh Dimention`))) (/ (`KismetMathLibrary.Conv_IntToDouble` _x) 2.0) 0.0)) (`KismetMathLibrary.FFloor` (+ (/ (.y `Tile Loc`) (.y (`self.Ice Cube Mesh Dimention`))) (/ (`KismetMathLibrary.Conv_IntToDouble` _y) 2.0) 0.0)))))

(fn `RemoveInstance`
  (params (Bucket :type "/Game/Blueprints/BPS_TileBucket Structure") (Index :type "IntPoint Structure"))
  (bind ((`InstancedMeshComponent_9_15013CAC4C513ECB4D65FB8969B052F8` _instancedmeshcomponent)) (break `/Game/Blueprints/BPS_TileBucket` Bucket))
  (bind _index (`self.CalculateIndex` Index))
  (`InstancedStaticMeshComponent.UpdateInstanceTransform` _instancedmeshcomponent _index (`KismetMathLibrary.MakeTransform` (`KismetMathLibrary.MakeVector` (.x (.location (`InstancedStaticMeshComponent.GetInstanceTransform` _instancedmeshcomponent _index false))) (.y (.location (`InstancedStaticMeshComponent.GetInstanceTransform` _instancedmeshcomponent _index false))) (`self.RemovalHeight`)) (.rotation (`InstancedStaticMeshComponent.GetInstanceTransform` _instancedmeshcomponent _index false)) (.scale (`InstancedStaticMeshComponent.GetInstanceTransform` _instancedmeshcomponent _index false))) false true true))

(fn `SetTileData`
  (params (TilePosition :type "IntPoint Structure") (TileData :type "/Game/Blueprints/BPS_IceTile Structure"))
  (bind (_x _y) (break `IntPoint` TilePosition))
  (`KismetArrayLibrary.Array_Set` (`self.MapData`) (+ _x (* _y (`.X` (break `IntPoint` (`self.Ice Map Size`))))) TileData true)
  (return))

(fn `UserConstructionScript`
  (bind (_x _y) (break `IntPoint` (`self.Ice Map Size`)))
  (for _index (range _x)
    (for _index_2 (range _y)
      (bind _tiletransform (`self.CalculateTileLocation` (make `IntPoint` _index _index_2)))
      (`InstancedStaticMeshComponent.AddInstance` (`self.MapSize`) _tiletransform))))