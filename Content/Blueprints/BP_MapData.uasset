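; BP_MapData holds the ice tile grid and player spawn locations for a map chosen by name from a lookup data table.
; Its construction script copies the row's size and spawn points, then unrolls the flat initial-state list row by row into tiles with position and zero damage.
; Helper functions map 2D coordinates to the flat array index to read, bounds-checked, or write tiles, and expose the grid size and all tile data.
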(fn `CalculateTileIndex`
  (params (TileLoc :type "IntPoint Structure (by ref)"))
  (returns (Index :type Integer))
  (bind (_x _y) (break `IntPoint` TileLoc))
  (return (+ _x (* _y (`.X` (break `IntPoint` (`self.Ice Map Size`)))))))

(fn `GetAllTileData`
  (returns (TileData :type "Array of /Game/Blueprints/BPS_IceTile Structure"))
  (return (`self.TileData`)))

(fn `GetIceMapSize`
  (returns (`Ice Map Size` :type "IntPoint Structure"))
  (return (`self.Ice Map Size`)))

(fn `GetTileData`
  (params (TileLoc :type "IntPoint Structure (by ref)"))
  (returns (Valid :type Boolean) (TileData :type "/Game/Blueprints/BPS_IceTile Structure") (Index :type Integer))
  (bind _tiledata (`self.TileData`))
  (bind _index (`self.CalculateTileIndex` TileLoc))
  (if (`KismetArrayLibrary.Array_IsValidIndex` _tiledata _index)
    (return true (`|GetArrayItem` _tiledata _index) _index)
    (else
      (return false (struct) _index))))

(fn `SetTileData`
  (params (TileLoc :type "IntPoint Structure (by ref)") (TileData :type "/Game/Blueprints/BPS_IceTile Structure (by ref)"))
  (bind _index (`self.CalculateTileIndex` TileLoc))
  (`KismetArrayLibrary.Array_Set` (`self.TileData`) _index TileData true)
  (return))

(fn `UserConstructionScript`
  (locals (BuildPoint :type "IntPoint Structure"))
  (bind (_x _y) (break `IntPoint` (`local.BuildPoint`)))
  (bind _returnvalue (+ _x 1))
  (`KismetArrayLibrary.Array_Clear` (`self.TileData`))
  (bind _returnvalue_2 (`|GetDataTableRow` (`self.MapDataLookupTable`) (`self.MapLookupName`))
    (:`then`
      (bind (_mapdimention _spawnlocations _initalstate) (break `/Game/Blueprints/BPS_Maps` _returnvalue_2))
      (set `self.Ice Map Size` _mapdimention)
      (set `self.PlayerSpawnLocations` _spawnlocations)
      (set `local.BuildPoint` (make `IntPoint` 0))
      (for _array_element _initalstate
        (`KismetArrayLibrary.Array_Add` (`self.TileData`) (make `/Game/Blueprints/BPS_IceTile` _array_element (`local.BuildPoint`)))
        (if (< _returnvalue (`.X` (break `IntPoint` (`self.Ice Map Size`))))
          (set `local.BuildPoint` (make `IntPoint` _returnvalue _y))
          (else
            (set `local.BuildPoint` (make `IntPoint` 0 (+ _y 1)))))))
    (:`RowNotFound`
      (`KismetSystemLibrary.PrintString` "Map Name not found" true true (struct :`R` 1.0 :`A` 1.0)))))