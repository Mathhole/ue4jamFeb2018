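; Ice map actor that renders a tile grid from MapDataClass and melts or heals tiles through damage.
; Each drawn ice state gets an instanced mesh holding every tile; state changes swap instance heights between zero and RemovalHeight.
; Hammer, player-melt and 3x3 mega-hammer events map locations to tiles for DamageTile, which steps states and saves map data.
; GetSpawnLocation hands out random, non-repeating spawn points above tiles.
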(event `self.ReceiveBeginPlay`
  (`InstancedStaticMeshComponent.ClearInstances` (`self.MapSize`))
  (`self.BucketGeneration`)
  (`self.GenerateInitalMesh`))

(event `HammerTime_Event`
  (params (HammerHitLoc :type "Vector Structure") (doesHeal :type Boolean))
  (bind _hammerdamage (`self.HammerDamage`))
  (bind _tile_index (`self.GetTileIndexFromLocation` HammerHitLoc))
  (`self.DamageTile` _tile_index (select `bool` doesHeal :`false` _hammerdamage :`true` (* -1 _hammerdamage))))

(event `PlayerMelt_Event`
  (params (PlayerLoc :type "Vector Structure") (doesHeal :type Boolean))
  (bind _standdamage (`self.StandDamage`))
  (bind _tile_index (`self.GetTileIndexFromLocation` PlayerLoc))
  (`self.DamageTile` _tile_index (select `bool` doesHeal :`false` _standdamage :`true` (* -1 _standdamage))))

(event `MegaHammerTime_Event`
  (params (HammerHitLoc :type "Vector Structure") (doesHeal :type Boolean))
  (bind _megahammerdamage (`self.MegaHammerDamage`))
  (bind _returnvalue (select `bool` doesHeal :`false` _megahammerdamage :`true` (* -1 _megahammerdamage)))
  ;[1 1 1] Megahammer Event - Pay no attention to the spegetti behind the curtain
  (bind _tile_index (`self.GetTileIndexFromLocation` HammerHitLoc))
  (`|ExecutionSequence`
    (:`then_0`
      (bind (_x _y) (break `IntPoint` _tile_index))
      (bind _returnvalue_2 (- _x 1))
      (`self.DamageTile` (make `IntPoint` _returnvalue_2 (- _y 1)) _returnvalue)
      (`self.DamageTile` (make `IntPoint` _returnvalue_2 _y) _returnvalue)
      (`self.DamageTile` (make `IntPoint` _returnvalue_2 (+ _y 1)) _returnvalue))
    (:`then_1`
      (`self.DamageTile` (make `IntPoint` _x (- _y 1)) _returnvalue)
      (`self.DamageTile` (make `IntPoint` _x _y) _returnvalue)
      (`self.DamageTile` (make `IntPoint` _x (+ _y 1)) _returnvalue))
    (:`then_2`
      (bind _returnvalue_3 (+ _x 1))
      (`self.DamageTile` (make `IntPoint` _returnvalue_3 (- _y 1)) _returnvalue)
      (`self.DamageTile` (make `IntPoint` _returnvalue_3 _y) _returnvalue)
      (`self.DamageTile` (make `IntPoint` _returnvalue_3 (+ _y 1)) _returnvalue))))

(fn `AddInstance`
  (params (Bucket :type "/Game/Blueprints/BPS_TileBucket Structure") (`Tile Loc` :type "IntPoint Structure"))
  (bind ((`StateMaterial_26_464E49D349390572013184AB0101E15B` _statematerial) (`InstancedMeshComponent_9_15013CAC4C513ECB4D65FB8969B052F8` _instancedmeshcomponent)) (break `/Game/Blueprints/BPS_TileBucket` Bucket))
  (bind _index (`/Game/Blueprints/BP_MapData.CalculateTileIndex` (`self.MapDataClass`) `Tile Loc`))
  (`/Engine/EditorBlueprintResources/StandardMacros.IsValid` _instancedmeshcomponent
    (:`Is Valid`
      (`InstancedStaticMeshComponent.UpdateInstanceTransform` _instancedmeshcomponent _index (`KismetMathLibrary.MakeTransform` (`KismetMathLibrary.MakeVector` (.x (.location (`InstancedStaticMeshComponent.GetInstanceTransform` _instancedmeshcomponent _index false))) (.y (.location (`InstancedStaticMeshComponent.GetInstanceTransform` _instancedmeshcomponent _index false)))) (.rotation (`InstancedStaticMeshComponent.GetInstanceTransform` _instancedmeshcomponent _index false)) (.scale (`InstancedStaticMeshComponent.GetInstanceTransform` _instancedmeshcomponent _index false))) false true true))))

(fn `BucketGeneration`
  (bind _enumvalue (foreach `/Game/Blueprints/BPE_IceState`)
    (:`LoopBody`
      (bind ((`State_20_C6E0F3984BD6CDFB172EC696CBA47F35` _state) (`StateMesh_2_BD42902149124139DA4A8DA67872F008` _statemesh) (`StateMaterial_26_464E49D349390572013184AB0101E15B` _statematerial) (`IsDrawn_17_F765C21744ACDBDEC1F79C925591F274` _isdrawn)) (break `/Game/Blueprints/BPS_TileBucket` (`|GetArrayItem` (`self.TileBuckets`) (`KismetMathLibrary.Conv_ByteToInt` _enumvalue))))
      (if _isdrawn
        (bind _returnvalue (`AddComponent|NODE_AddInstancedStaticMeshComponent-0`))
        (`StaticMeshComponent.SetStaticMesh` _returnvalue _statemesh)
        (`PrimitiveComponent.SetMaterial` _returnvalue 0 (`.MaterialInterface` (break `StaticMaterial` _statematerial)))
        (`SceneComponent.K2_AttachToComponent` _returnvalue (`self.IceSegments`) "None" "SnapToTarget" "SnapToTarget" "SnapToTarget" true)
        (`KismetArrayLibrary.Array_Set` (`self.TileBuckets`) (`KismetMathLibrary.Conv_ByteToInt` _state) (make `/Game/Blueprints/BPS_TileBucket` _state _statemesh _statematerial _returnvalue))))))

(fn `CalculateTileLocation`
  (params (TileLoc :type "IntPoint Structure"))
  (returns (TileTransform :type "Transform Structure"))
  (bind (_x _y) (break `IntPoint` TileLoc))
  (bind _x_2 (.x (`self.Ice Cube Mesh Dimention`)))
  (bind _y_2 (.y (`self.Ice Cube Mesh Dimention`)))
  (bind _ice_map_size (`/Game/Blueprints/BP_MapData.GetIceMapSize` (`self.MapDataClass`)))
  (bind (_x_3 _y_3) (break `IntPoint` _ice_map_size))
  (return (`KismetMathLibrary.Conv_VectorToTransform` (`KismetMathLibrary.MakeVector` (+ (- (* _x _x_2) (/ (* _x_3 _x_2) 2.0)) (/ _x_2 2.0)) (+ (- (* _y _y_2) (/ (* _y_3 _y_2) 2.0)) (/ _y_2 2.0))))))

(fn `DamageTile`
  (params (TilePosition :type "IntPoint Structure") (Damage :type "Float (double-precision)"))
  (locals (CurIceState :type "/Game/Blueprints/BPE_IceState Enum") (TempDamage :type "Float (double-precision)") (TilePos :type "IntPoint Structure"))
  (bind (_x _y) (break `IntPoint` TilePosition))
  (bind _tilepos (`local.TilePos`))
  (bind (_valid _tiledata) (`/Game/Blueprints/BP_MapData.GetTileData` (`self.MapDataClass`) TilePosition))
  (if _valid
    (bind (_state _position _totaldamage) (break `/Game/Blueprints/BPS_IceTile` _tiledata))
    (set `local.CurIceState` _state)
    (set `local.TilePos` _position)
    (bind _output_get (set `local.TempDamage` (+ Damage _totaldamage)))
    (if (>= _output_get (`self.MaximumDamage`))
      ;[1 1 1] State Down
      (while (and (>= (`local.TempDamage`) (`self.MaximumDamage`)) (`|EnumInequality` (`local.CurIceState`) "NewEnumerator6"))
        (set `local.TempDamage` (- (`local.TempDamage`) (`self.MaximumDamage`)))
        (bind _newstate (`self.StateChangeDown` (`local.CurIceState`) (`local.TilePos`)))
        (set `local.CurIceState` _newstate))
      (elif (< _output_get 0.0)
        ;[1 1 1] State Up
        (while (and (< (`local.TempDamage`) 0.0) true)
          (if (`|EnumEquality` (`local.CurIceState`) "NewEnumerator0")
            (set `local.TempDamage` 0.0)
            (else
              (set `local.TempDamage` (+ (`local.TempDamage`) (`self.MaximumDamage`)))
              (bind _newstate_2 (`self.StateChangeUp` (`local.CurIceState`) (`local.TilePos`)))
              (set `local.CurIceState` _newstate_2))))))
    ;[1 1 1] Update Tile Data
    (`/Game/Blueprints/BP_MapData.SetTileData` (`self.MapDataClass`) _tilepos (make `/Game/Blueprints/BPS_IceTile` (`local.CurIceState`) _tilepos (`local.TempDamage`)))
    (else
      (`KismetSystemLibrary.PrintString` (`KismetStringLibrary.Concat_StrStr` "TileDamage: Invalid Tile (" (`KismetStringLibrary.Conv_IntToString` _x) " : " (`KismetStringLibrary.Conv_IntToString` _y) ")")))))

(fn `GenerateInitalMesh`
  (`|ExecutionSequence`
    (:`then_0`
      ;[1 1 1] Distribute Into Buckets
      (bind _tiledata (`/Game/Blueprints/BP_MapData.GetAllTileData` (`self.MapDataClass`)))
      (for (_array_element _array_index) _tiledata
        (bind (_state _position) (break `/Game/Blueprints/BPS_IceTile` _array_element))
        (if (`.IsDrawn_17_F765C21744ACDBDEC1F79C925591F274` (break `/Game/Blueprints/BPS_TileBucket` (`|GetArrayItem` (`self.TileBuckets`) (`KismetMathLibrary.Conv_ByteToInt` _state))))
          (`KismetArrayLibrary.Array_Set` _tiledata _array_index (make `/Game/Blueprints/BPS_IceTile` _state _position) true))))
    (:`then_1`
      ;[1 1 1] Generate Tile Instances
      (bind _enumvalue (foreach `/Game/Blueprints/BPE_IceState`)
        (:`LoopBody`
          (bind _ice_map_size (`/Game/Blueprints/BP_MapData.GetIceMapSize` (`self.MapDataClass`)))
          (bind ((`StateMaterial_26_464E49D349390572013184AB0101E15B` _statematerial) (`InstancedMeshComponent_9_15013CAC4C513ECB4D65FB8969B052F8` _instancedmeshcomponent) (`IsDrawn_17_F765C21744ACDBDEC1F79C925591F274` _isdrawn)) (break `/Game/Blueprints/BPS_TileBucket` (`|GetArrayItem` (`self.TileBuckets`) (`KismetMathLibrary.Conv_ByteToInt` _enumvalue))))
          (if _isdrawn
            (bind (_x _y) (break `IntPoint` _ice_map_size))
            (for _index (range _y)
              (for _index_2 (range _x)
                (bind _intpoint (make `IntPoint` _index_2 _index))
                (bind _index_3 (`/Game/Blueprints/BP_MapData.CalculateTileIndex` (`self.MapDataClass`) _intpoint))
                (bind _tiledata_2 (`/Game/Blueprints/BP_MapData.GetAllTileData` (`self.MapDataClass`)))
                (bind _tiletransform (`self.CalculateTileLocation` _intpoint))
                (`InstancedStaticMeshComponent.AddInstance` _instancedmeshcomponent (`KismetMathLibrary.MakeTransform` (`KismetMathLibrary.MakeVector` (.x (.location _tiletransform)) (.y (.location _tiletransform)) (select `bool` (`|EnumEquality` (`.State_7_25813F964726E9687C2E05B5FFACDAAC` (break `/Game/Blueprints/BPS_IceTile` (`|GetArrayItem` _tiledata_2 _index_3))) _enumvalue) :`false` (`self.RemovalHeight`))) (.rotation _tiletransform) (.scale _tiletransform)))))))))))

(fn `GetNextIceState`
  (params (OldIceState :type "/Game/Blueprints/BPE_IceState Enum" :default "NewEnumerator0"))
  (returns (NextIceState :type "/Game/Blueprints/BPE_IceState Enum") (PrevIceState :type "/Game/Blueprints/BPE_IceState Enum") (OrignalBucket :type "/Game/Blueprints/BPS_TileBucket Structure") (NextBucket :type "/Game/Blueprints/BPS_TileBucket Structure") (PrevBucket :type "/Game/Blueprints/BPS_TileBucket Structure"))
  (bind _tilebuckets (`self.TileBuckets`))
  (bind _output (`|GetArrayItem` _tilebuckets))
  (bind _output_2 (`|GetArrayItem` _tilebuckets 3))
  (bind _output_3 (`|GetArrayItem` _tilebuckets 4))
  (bind _output_4 (`|GetArrayItem` _tilebuckets 5))
  (bind _output_5 (`|GetArrayItem` _tilebuckets 6))
  (bind _output_6 (`|GetArrayItem` _tilebuckets 2))
  (bind _output_7 (`|GetArrayItem` _tilebuckets 1))
  (return (select `/Game/Blueprints/BPE_IceState` OldIceState :`NewEnumerator0` "NewEnumerator1" :`NewEnumerator1` "NewEnumerator2" :`NewEnumerator2` "NewEnumerator3" :`NewEnumerator3` "NewEnumerator4" :`NewEnumerator4` "NewEnumerator5" :`NewEnumerator5` "NewEnumerator6" :`NewEnumerator6` "NewEnumerator6" :!type "/Game/Blueprints/BPE_IceState Enum") (select `/Game/Blueprints/BPE_IceState` OldIceState :`NewEnumerator0` "NewEnumerator0" :`NewEnumerator1` "NewEnumerator0" :`NewEnumerator2` "NewEnumerator1" :`NewEnumerator3` "NewEnumerator2" :`NewEnumerator4` "NewEnumerator3" :`NewEnumerator5` "NewEnumerator4" :`NewEnumerator6` "NewEnumerator5" :!type "/Game/Blueprints/BPE_IceState Enum") (select `/Game/Blueprints/BPE_IceState` OldIceState :`NewEnumerator0` _output :`NewEnumerator1` _output_7 :`NewEnumerator2` _output_6 :`NewEnumerator3` _output_2 :`NewEnumerator4` _output_3 :`NewEnumerator5` _output_4 :`NewEnumerator6` _output_5) (select `/Game/Blueprints/BPE_IceState` OldIceState :`NewEnumerator0` _output_7 :`NewEnumerator1` _output_6 :`NewEnumerator2` _output_2 :`NewEnumerator3` _output_3 :`NewEnumerator4` _output_4 :`NewEnumerator5` _output_5 :`NewEnumerator6` _output_5) (select `/Game/Blueprints/BPE_IceState` OldIceState :`NewEnumerator0` _output :`NewEnumerator1` _output :`NewEnumerator2` _output_7 :`NewEnumerator3` _output_6 :`NewEnumerator4` _output_2 :`NewEnumerator5` _output_3 :`NewEnumerator6` _output_4)))

(fn `GetSpawnLocation`
  (returns (SpawnLocation :type "Transform Structure"))
  (locals (RandIndex :type Integer))
  (bind _playerspawnlocations (`/Game/Blueprints/BP_MapData.PlayerSpawnLocations` (`self.MapDataClass`)))
  (bind _output_get (set `local.RandIndex` (`KismetMathLibrary.RandomInteger` (`KismetArrayLibrary.Array_Length` _playerspawnlocations))))
  (bind _tiletransform (`self.CalculateTileLocation` (`|GetArrayItem` _playerspawnlocations _output_get)))
  (`KismetArrayLibrary.Array_Remove` _playerspawnlocations _output_get)
  (return (`KismetMathLibrary.ComposeTransforms` _tiletransform (`KismetMathLibrary.MakeTransform` (0.0 0.0 100.0)))))

(fn `GetTileIndexFromLocation`
  (params (`Tile Loc` :type "Vector Structure"))
  (returns (`Tile Index` :type "IntPoint Structure"))
  (bind _ice_map_size (`/Game/Blueprints/BP_MapData.GetIceMapSize` (`self.MapDataClass`)))
  (bind (_x _y) (break `IntPoint` _ice_map_size))
  (return (make `IntPoint` (`KismetMathLibrary.FFloor` (+ (/ (.x `Tile Loc`) (.x (`self.Ice Cube Mesh Dimention`))) (/ (`KismetMathLibrary.Conv_IntToDouble` _x) 2.0) 0.0)) (`KismetMathLibrary.FFloor` (+ (/ (.y `Tile Loc`) (.y (`self.Ice Cube Mesh Dimention`))) (/ (`KismetMathLibrary.Conv_IntToDouble` _y) 2.0) 0.0)))))

(fn `RemoveInstance`
  (params (Bucket :type "/Game/Blueprints/BPS_TileBucket Structure") (`Tile Loc` :type "IntPoint Structure"))
  (bind ((`StateMaterial_26_464E49D349390572013184AB0101E15B` _statematerial) (`InstancedMeshComponent_9_15013CAC4C513ECB4D65FB8969B052F8` _instancedmeshcomponent)) (break `/Game/Blueprints/BPS_TileBucket` Bucket))
  (bind _index (`/Game/Blueprints/BP_MapData.CalculateTileIndex` (`self.MapDataClass`) `Tile Loc`))
  (`/Engine/EditorBlueprintResources/StandardMacros.IsValid` _instancedmeshcomponent
    (:`Is Valid`
      (`InstancedStaticMeshComponent.UpdateInstanceTransform` _instancedmeshcomponent _index (`KismetMathLibrary.MakeTransform` (`KismetMathLibrary.MakeVector` (.x (.location (`InstancedStaticMeshComponent.GetInstanceTransform` _instancedmeshcomponent _index false))) (.y (.location (`InstancedStaticMeshComponent.GetInstanceTransform` _instancedmeshcomponent _index false))) (`self.RemovalHeight`)) (.rotation (`InstancedStaticMeshComponent.GetInstanceTransform` _instancedmeshcomponent _index false)) (.scale (`InstancedStaticMeshComponent.GetInstanceTransform` _instancedmeshcomponent _index false))) false true true))))

(fn `StateChangeDown`
  (params (IceState :type "/Game/Blueprints/BPE_IceState Enum" :default "NewEnumerator0") (TileLoc :type "IntPoint Structure"))
  (returns (NewState :type "/Game/Blueprints/BPE_IceState Enum"))
  (bind (_nexticestate _previcestate _orignalbucket _nextbucket) (`self.GetNextIceState` IceState))
  (`self.AddInstance` _nextbucket TileLoc)
  (`self.RemoveInstance` _orignalbucket TileLoc)
  (return _nexticestate))

(fn `StateChangeUp`
  (params (IceState :type "/Game/Blueprints/BPE_IceState Enum" :default "NewEnumerator0") (TileLoc :type "IntPoint Structure"))
  (returns (NewState :type "/Game/Blueprints/BPE_IceState Enum"))
  (bind (_nexticestate _previcestate _orignalbucket _nextbucket _prevbucket) (`self.GetNextIceState` IceState))
  (`self.AddInstance` _prevbucket TileLoc)
  (`self.RemoveInstance` _orignalbucket TileLoc)
  (return _previcestate))

(fn `UserConstructionScript`
  (bind _ice_map_size (`/Game/Blueprints/BP_MapData.GetIceMapSize` (`self.MapDataClass`)))
  (bind (_x _y) (break `IntPoint` _ice_map_size))
  (for _index (range _x)
    (for _index_2 (range _y)
      (bind _tiletransform (`self.CalculateTileLocation` (make `IntPoint` _index _index_2)))
      (`InstancedStaticMeshComponent.AddInstance` (`self.MapSize`) _tiletransform))))