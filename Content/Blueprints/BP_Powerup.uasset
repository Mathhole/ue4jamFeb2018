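; BP_Powerup is a powerup actor encased in an ice cage that travels to a target location and takes hits to uncover.
; Tick moves it toward TargetLocation at TravelSpeed, snapping into place and stopping on arrival.
; Construction creates a dynamic ice material colored by HitsRemaining.
; HandleHit decrements that count, recoloring the ice from IceColors, then hides the cage and disables its collision once the count drops below zero.
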(event `self.ReceiveTick`
  (params (DeltaSeconds :type "Float (single-precision)"))
  (`self.MoveTowardTarget` DeltaSeconds))

(fn `HandleHit`
  (bind _result (`/Engine/EditorBlueprintResources/StandardMacros.DecrementInt` (`self.HitsRemaining`))
    (:`  `
      (if (< _result 0)
        (`SceneComponent.SetVisibility` (`self.IcyCage`) false false)
        (`PrimitiveComponent.SetCollisionEnabled` (`self.IcyCage`) "NoCollision")
        (else
          (`MaterialInstanceDynamic.SetVectorParameterValue` (`self.IceMat`) "IceColor" (`|GetArrayItem` (`self.IceColors`) _result)))))))

(fn `MoveTowardTarget`
  (params (DT :type "Float (double-precision)"))
  (if (`self.Arrived`)
    _
    (elif (< (`KismetMathLibrary.VSize` (- (`self.TargetLocation`) (`self.K2_GetActorLocation`))) (* (`local.DT`) (`self.TravelSpeed`)))
      (`self.K2_SetActorLocation` (`self.TargetLocation`))
      (set `self.Arrived` true)
      (else
        (`self.K2_SetActorLocation` (+ (`self.K2_GetActorLocation`) (* (`KismetMathLibrary.Normal` (- (`self.TargetLocation`) (`self.K2_GetActorLocation`))) (* (`local.DT`) (`self.TravelSpeed`)))))))))

(fn `UserConstructionScript`
  (bind _returnvalue (`PrimitiveComponent.CreateDynamicMaterialInstance` (`self.IcyCage`) 0 "/Game/materials/m_iceblock_solid.m_iceblock_solid"))
  (set `self.IceMat` _returnvalue)
  (`MaterialInstanceDynamic.SetVectorParameterValue` (`self.IceMat`) "IceColor" (`|GetArrayItem` (`self.IceColors`) (`self.HitsRemaining`))))